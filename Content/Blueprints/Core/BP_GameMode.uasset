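; BP_GameMode is a game mode Blueprint that exercises the session state and time tick features of TinyRogueGameState.
; On PostInitGame it binds handlers to both game state delegates, then switches the session from InProgress to Paused and back using timed delays.
; The handlers only print the tick time and new state to screen, so the graph behaves as a debug test sequence.
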(event Custom|OnTimeTickDelegate_Event
  (params (Time :type Timespan%20Structure%20%28by%20ref%29))
  (Development|PrintString (Class|UtilityFunctionsLibrary|ToString(Timespan) Time) true true "(R=0.000000,G=0.660000,B=1.000000,A=1.000000)" 1.0))

(event Custom|OnGameSessionStateChangedDelegate_Event
  (params (NewGameSessionState :type EGameSessionState%20Enum%20%28by%20ref%29 :default "WaitingToStart"))
  (Development|PrintString (Utilities|String|EnumtoString NewGameSessionState) true true "(R=0.000000,G=1.000000,B=0.000000,A=1.000000)" 5.0))

(event EventBeginPlay)

(event EventPostInitGame
  (bind _astiny_rogue_game_state (Utilities|Casting|CastToTinyRogueGameState (Game|GetGameState)))
  (EventDispatchers|AssignOnTimeTickDelegate _astiny_rogue_game_state (delegate Custom|OnTimeTickDelegate_Event))
  (EventDispatchers|AssignOnGameSessionStateChangedDelegate _astiny_rogue_game_state (delegate Custom|OnGameSessionStateChangedDelegate_Event))
  (Class|TinyRogueGameState|SetGameSessionState _astiny_rogue_game_state "InProgress")
  (Utilities|FlowControl|Delay 3.0)
  (Class|TinyRogueGameState|SetGameSessionState _astiny_rogue_game_state "Paused")
  (Utilities|FlowControl|Delay 3.0)
  (Class|TinyRogueGameState|SetGameSessionState _astiny_rogue_game_state "InProgress"))

(fn ConstructionScript)