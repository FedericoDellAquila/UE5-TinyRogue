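; BP_TestCommand is a test command Blueprint that finishes itself after a short delay.
; Execute calls the parent, then starts a one-shot timer whose event calls Finish.
; A damage handler would also Finish and dequeue from the command subsystem, but its binding to the player is disconnected.
; Update is an empty override, with its parent call and DeltaTime print left unwired.
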(event Custom|OnTakeAnyDamage_Event
  (params (DamagedActor :type Actor%20Object%20Reference) (Damage :type Float%20%28single-precision%29) (DamageType :type Damage%20Type%20Object%20Reference) (InstigatedBy :type Controller%20Object%20Reference) (DamageCauser :type Actor%20Object%20Reference))
  (Class|Command|Finish)
  (Class|CommandSubsystem|Dequeue (Class|Command|GetCommandSubsystem)))

(event Custom|CustomEvent
  (Class|Command|Finish))

(event EventExecute
  (|CallParentFunction)
  (Utilities|Time|SetTimerbyEvent (delegate Custom|CustomEvent) 3.0))

(event EventUpdate
  (params (DeltaTime :type Float%20%28single-precision%29)))